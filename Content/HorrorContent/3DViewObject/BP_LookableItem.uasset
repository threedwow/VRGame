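; Interactable world item that the player can pick up to inspect in a 3D view widget.
; Interaction passes its mesh, material and scale to the character's viewer, with take/put-back sounds and optional hiding while held.
; Radius events toggle the prompt if CanTakeItem, using a screen widget in third person or world widget in first.
; Construction applies the mesh and material; a helper sets the prompt's name per player mode.
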(event Custom|PutBack
  ;[1 1 1] Show Item and play sound
  (Audio|PlaySound2D (Variables|Default|GetPutSound))
  (if (Variables|Default|GetHideWhenTookItem)
    (Rendering|SetVisibility (Variables|Default|GetItem) true false)))

(event EventPlayerEnterRadius
  (params (Character :type Third%20Person%20Character%20Object%20Reference))
  ;[1 1 1] Setting up widget depending on players state
  (if (Variables|Default|GetCanTakeItem?)
    (CallFunction|NewWidgetState Character true)))

(event EventPlayerLeaveRadius
  (params (Chareacter :type Third%20Person%20Character%20Object%20Reference))
  ;[1 1 1] Setting up widget depending on players state
  (if (Variables|Default|GetCanTakeItem?)
    (CallFunction|NewWidgetState Chareacter false)))

(event EventInteractwith
  (params (Character :type Third%20Person%20Character%20Object%20Reference))
  ;[1 1 1] Open 3DViewWidget
  (Default|Open3DViewItem Character (Variables|MeshSettings|GetNewMesh) (Variables|MeshSettings|GetMaterial) self (Variables|MeshSettings|GetScale))
  (Audio|PlaySound2D (Variables|Default|GetTakeSound))
  ;;[1 1 1] Hide Item when took
  (if (Variables|Default|GetHideWhenTookItem)
    (Rendering|SetVisibility (Variables|Default|GetItem) false false)))

(fn ConstructionScript
  (bind _item (Variables|Default|GetItem))
  (Components|StaticMesh|SetStaticMesh _item (Variables|MeshSettings|GetNewMesh))
  (Rendering|Material|SetMaterial _item 0 (Variables|MeshSettings|GetMaterial)))

(fn NewWidgetState
  (params (Player :type Third%20Person%20Character%20Object%20Reference) (New%20hidden :type Boolean))
  ;[1 1 1] Setting up widget
  (switch Utilities|FlowControl|Switch|SwitchonEPlayer (Variables|/Game/HorrorContent/MainBlueprints/ThirdPersonCharacter.ThirdPersonCharacter_C|GetPlayerMode Player)
    (:NewEnumerator0
      ;;[1 1 1] Visibility for third person widget
      (if New%20hidden
        (Widget|SetVisibility (Variables|/Game/HorrorContent/MainBlueprints/ThirdPersonCharacter.ThirdPersonCharacter_C|GetInteractionWidgetScreen Player) "Visible")
        (else
          (Widget|SetVisibility (Variables|/Game/HorrorContent/MainBlueprints/ThirdPersonCharacter.ThirdPersonCharacter_C|GetInteractionWidgetScreen Player) "Hidden"))))
    (:NewEnumerator1
      ;;[1 1 1] Visibility for first person widget
      (if New%20hidden
        (Development|SetHiddeninGame (Variables|Default|GetInteractionWidget) false false)
        (else
          (Development|SetHiddeninGame (Variables|Default|GetInteractionWidget) true false))))))

(fn ChangeNameinWidget
  (params (Character :type Third%20Person%20Character%20Object%20Reference) (Widget%20World :type Widget%20Component%20Object%20Reference) (Widget%20Screen :type W%20Interaction%20Screen%20Object%20Reference) (Name :type Text))
  (switch Utilities|FlowControl|Switch|SwitchonEPlayer (Variables|/Game/HorrorContent/MainBlueprints/ThirdPersonCharacter.ThirdPersonCharacter_C|GetPlayerMode Character)
    (:NewEnumerator0
      (Rendering|Components|TextRender|SetText (Variables|/Game/HorrorContent/Widgets/W_InteractionScreen.W_InteractionScreen_C|GetName Widget%20Screen) Name))
    (:NewEnumerator1
      (bind _asw_interaction_world (Utilities|Casting|CastToW_InteractionWorld (UserInterface|GetUserWidgetObject Widget%20World)))
      (Rendering|Components|TextRender|SetText (Variables|/Game/HorrorContent/Widgets/W_InteractionWorld.W_InteractionWorld_C|GetName _asw_interaction_world) Name))))