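; Throwable item actor that launches itself as a physics object when play begins, as either a static or destructible mesh.
; The construction script assigns the configured assets to both mesh components.
; On BeginPlay, MeshState selects the component that receives an impulse at the actor location, scaled from the actor's current velocity by MultiplyVelocity, and wakes its rigid body.
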(event EventBeginPlay
  ;[1 1 1] GiveImpulseToObject
  (CallFunction|SetImpulsebyMeshMode (Variables|Default|GetMultiplyVelocity) (Variables|Default|GetItem) (Variables|Default|GetDestructibleItem)))

(fn ConstructionScript
  (Components|StaticMesh|SetStaticMesh (Variables|Default|GetItem) (Variables|Default|GetStaticMesh))
  (Class|DestructibleComponent|SetDestructibleMesh (Variables|Default|GetDestructibleItem) (Variables|Default|GetDestuctible)))

(fn SetImpulsebyMeshMode
  (params (MVelocity :type Vector) (StaticMesh :type Primitive%20Component%20Object%20Reference) (Destructible :type Destructible%20Component%20Object%20Reference))
  ;[1 1 1] Choose to what object give impulse
  (switch Utilities|FlowControl|Switch|SwitchonEThrowItem (Variables|Default|GetMeshState)
    (:NewEnumerator0
      ;;[1 1 1] Set start impulse to static mesh
      (Physics|AddImpulseatLocation StaticMesh (* (Transformation|GetVelocity) MVelocity) (Transformation|GetActorLocation) "None")
      (Class|PrimitiveComponent|WakeRigidBody StaticMesh "None"))
    (:NewEnumerator1
      ;;[1 1 1] Set start impulse to destructible
      (Physics|AddImpulseatLocation Destructible (* (Transformation|GetVelocity) MVelocity) (Transformation|GetActorLocation) "None")
      (Class|PrimitiveComponent|WakeRigidBody Destructible "None"))))