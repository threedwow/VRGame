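; BP_KeepItem is a pickup the player takes into their inventory.
; Entering its radius shows a prompt labeled with UseText; leaving hides it and restores "Open", using the screen widget in third person or the world widget in first person.
; Interacting routes through server and all-clients events that add the item to the character's inventory and destroy the actor, gated by CanTakeItem.
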(event Custom|TakeObject%20-ALL
  (params (Character :type Third%20Person%20Character%20Object%20Reference))
  ;[1 1 1] Give item to player
  (if (Variables|Default|GetCanTakeItem?)
    (Utilities|Array|Add (Variables|/Game/HorrorContent/MainBlueprints/ThirdPersonCharacter.ThirdPersonCharacter_C|GetInventory Character) (Variables|Default|GetItemToGivePlayer))
    (Actor|DestroyActor)))

(event Custom|TakeObject%20-Server
  (params (Character :type Third%20Person%20Character%20Object%20Reference))
  ;[1 1 1] Give item to player
  (CallFunction|TakeObject-ALL Character))

(event EventBeginPlay
  ;[1 1 1] Set player Reference
  (bind _asthird_person_character (Utilities|Casting|CastToThirdPersonCharacter (Game|GetPlayerCharacter 0)))
  (Variables|Default|SetPlayer%20Reference _asthird_person_character))

(event EventPlayerEnterRadius
  (params (Character :type Third%20Person%20Character%20Object%20Reference))
  (bind _player_reference (Variables|Default|GetPlayer%20Reference))
  ;[1 1 1] Setting up widget depending on players state
  (if (Variables|Default|GetCanTakeItem?)
    (CallFunction|NewWidgetState Character true)
    ;[1 1 1] Set widgets variable name to UseText
    (CallFunction|ChangeNameinWidget _player_reference (Variables|Default|GetInteractionWidget) (Variables|/Game/HorrorContent/MainBlueprints/ThirdPersonCharacter.ThirdPersonCharacter_C|GetInteractionWidgetScreen _player_reference) (Variables|Default|GetUseText))))

(event EventPlayerLeaveRadius
  (params (Chareacter :type Third%20Person%20Character%20Object%20Reference))
  (bind _player_reference (Variables|Default|GetPlayer%20Reference))
  ;[1 1 1] Setting up widget depending on players state
  (if (Variables|Default|GetCanTakeItem?)
    (CallFunction|NewWidgetState Chareacter false)
    ;[1 1 1] Set widgets variable name to casual "Open"
    (CallFunction|ChangeNameinWidget _player_reference (Variables|Default|GetInteractionWidget) (Variables|/Game/HorrorContent/MainBlueprints/ThirdPersonCharacter.ThirdPersonCharacter_C|GetInteractionWidgetScreen _player_reference) "Open")))

(event EventInteractwith
  (params (Character :type Third%20Person%20Character%20Object%20Reference))
  ;[1 1 1] Give item to player
  (CallFunction|TakeObject-Server Character))

(fn ConstructionScript)

(fn NewWidgetState
  (params (Player :type Third%20Person%20Character%20Object%20Reference) (New%20hidden :type Boolean))
  ;[1 1 1] Setting up widget
  (switch Utilities|FlowControl|Switch|SwitchonEPlayer (Variables|/Game/HorrorContent/MainBlueprints/ThirdPersonCharacter.ThirdPersonCharacter_C|GetPlayerMode Player)
    (:NewEnumerator0
      ;;[1 1 1] Visibility for third person widget
      (if New%20hidden
        (Widget|SetVisibility (Variables|/Game/HorrorContent/MainBlueprints/ThirdPersonCharacter.ThirdPersonCharacter_C|GetInteractionWidgetScreen Player) "Visible")
        (else
          (Widget|SetVisibility (Variables|/Game/HorrorContent/MainBlueprints/ThirdPersonCharacter.ThirdPersonCharacter_C|GetInteractionWidgetScreen Player) "Hidden"))))
    (:NewEnumerator1
      ;;[1 1 1] Visibility for first person widget
      (if New%20hidden
        (Development|SetHiddeninGame (Variables|Default|GetInteractionWidget) false false)
        (else
          (Development|SetHiddeninGame (Variables|Default|GetInteractionWidget) true false))))))

(fn ChangeNameinWidget
  (params (Character :type Third%20Person%20Character%20Object%20Reference) (Widget%20World :type Widget%20Component%20Object%20Reference) (Widget%20Screen :type W%20Interaction%20Screen%20Object%20Reference) (Name :type Text))
  (switch Utilities|FlowControl|Switch|SwitchonEPlayer (Variables|/Game/HorrorContent/MainBlueprints/ThirdPersonCharacter.ThirdPersonCharacter_C|GetPlayerMode Character)
    (:NewEnumerator0
      (Rendering|Components|TextRender|SetText (Variables|/Game/HorrorContent/Widgets/W_InteractionScreen.W_InteractionScreen_C|GetName Widget%20Screen) Name))
    (:NewEnumerator1
      (bind _asw_interaction_world (Utilities|Casting|CastToW_InteractionWorld (UserInterface|GetUserWidgetObject Widget%20World)))
      (Rendering|Components|TextRender|SetText (Variables|/Game/HorrorContent/Widgets/W_InteractionWorld.W_InteractionWorld_C|GetName _asw_interaction_world) Name))))