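; BP_Door is an interactable door for the horror content that characters open and close, with configurable meshes and start angle.
; Interaction toggles a timeline that plays or reverses to rotate the door, blocking reuse while it moves.
; Each toggle plays a 2D sound and can emit MakeNoise attributed to the player pawn.
; The prompt's visibility and text target a screen widget in third person or a world widget in first person.
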(event Custom|OpenDoor
  ;[1 1 1] Door movement timeline
  (Variables|Default|SetOpened? true)
  (Audio|PlaySound2D (Variables|Default|GetOpenDoorSound))
  (CallFunction|MakeDoorNoise (Variables|Noise|GetCanMakeNoise) (Transformation|GetActorLocation))
  (bind _value (Timeline|DoorOpenClose Play)
    (:Update
      (Transformation|SetRelativeRotation (Variables|Default|GetDoor) (Math|Rotator|MakeRotator 0.0 0.0 (- (select (Variables|Default|GetPositiveDirection?) 1.8e+02 -9e+01) _value)) false false)
      (Variables|Default|SetCanUseDoor? false))
    (:Finished
      (Variables|Default|SetCanUseDoor? true))))

(event Custom|CloseDoor
  ;[1 1 1] Door movement timeline
  (Variables|Default|SetOpened? false)
  (Audio|PlaySound2D (Variables|Default|GetCloseDoorSound))
  (CallFunction|MakeDoorNoise (Variables|Noise|GetCanMakeNoise) (Transformation|GetActorLocation))
  (bind _value (Timeline|DoorOpenClose Reverse)
    (:Update
      (Transformation|SetRelativeRotation (Variables|Default|GetDoor) (Math|Rotator|MakeRotator 0.0 0.0 (- (select (Variables|Default|GetPositiveDirection?) 1.8e+02 -9e+01) _value)) false false)
      (Variables|Default|SetCanUseDoor? false))
    (:Finished
      (Variables|Default|SetCanUseDoor? true))))

(event Custom|MakeDoorNoise
  (params (NeedToMakeNoise? :type Boolean) (NoiseLocation :type Vector))
  ;[1 1 1] DoorMakeNoise
  (if NeedToMakeNoise?
    (Class|Actor|MakeNoise (Variables|Noise|GetNoise) (Game|Player|GetPlayerPawn 0) NoiseLocation 0.0 "None")))

(event EventPlayerEnterRadius
  (params (Character :type Third%20Person%20Character%20Object%20Reference))
  ;[1 1 1] Setting up widget depending on players state
  (if (Variables|Default|GetCanOpenOrCloseDoor?)
    (CallFunction|NewWidgetState Character true)))

(event EventPlayerLeaveRadius
  (params (Chareacter :type Third%20Person%20Character%20Object%20Reference))
  ;[1 1 1] Setting up widget depending on players state
  (if (Variables|Default|GetCanOpenOrCloseDoor?)
    (CallFunction|NewWidgetState Chareacter false)))

(event EventInteractwith
  (params (Character :type Third%20Person%20Character%20Object%20Reference))
  (bind _interactionwidgetscreen (Variables|/Game/HorrorContent/MainBlueprints/ThirdPersonCharacter.ThirdPersonCharacter_C|GetInteractionWidgetScreen Character))
  (bind _interactionwidget (Variables|Default|GetInteractionWidget))
  ;[1 1 1] Open or close door when player interact
  (if (Variables|Default|GetCanOpenOrCloseDoor?)
    ;;[1 1 1] Player can not use door while timeline is played
    (if (Variables|Default|GetCanUseDoor?)
      (if (Variables|Default|GetOpened?)
        ;;[1 1 1] Change widgets state and close door
        (CallFunction|CloseDoor)
        (CallFunction|ChangeNameinWidget Character _interactionwidget _interactionwidgetscreen (Utilities|Array|Get(acopy) (Variables|Default|GetUseText) 1))
        (else
          ;;[1 1 1] Change widgets state and close door
          (CallFunction|OpenDoor)
          (CallFunction|ChangeNameinWidget Character _interactionwidget _interactionwidgetscreen (Utilities|Array|Get(acopy) (Variables|Default|GetUseText))))))))

(fn ConstructionScript
  (Transformation|SetRelativeRotation (Variables|Default|GetDoor) (Math|Rotator|MakeRotator 0.0 0.0 (Variables|Default|GetStartAngle)) false false)
  (Components|StaticMesh|SetStaticMesh (Variables|Default|GetDoor) (Variables|Default|GetNewDoor))
  (Components|StaticMesh|SetStaticMesh (Variables|Default|GetDoorFrame) (Variables|Default|GetNewFrame)))

(fn NewWidgetState
  (params (Player :type Third%20Person%20Character%20Object%20Reference) (New%20hidden :type Boolean))
  ;[1 1 1] Setting up widget
  (switch Utilities|FlowControl|Switch|SwitchonEPlayer (Variables|/Game/HorrorContent/MainBlueprints/ThirdPersonCharacter.ThirdPersonCharacter_C|GetPlayerMode Player)
    (:NewEnumerator0
      ;;[1 1 1] Visibility for third person widget
      (if New%20hidden
        (Widget|SetVisibility (Variables|/Game/HorrorContent/MainBlueprints/ThirdPersonCharacter.ThirdPersonCharacter_C|GetInteractionWidgetScreen Player) "Visible")
        (else
          (Widget|SetVisibility (Variables|/Game/HorrorContent/MainBlueprints/ThirdPersonCharacter.ThirdPersonCharacter_C|GetInteractionWidgetScreen Player) "Hidden"))))
    (:NewEnumerator1
      ;;[1 1 1] Visibility for first person widget
      (if New%20hidden
        (Development|SetHiddeninGame (Variables|Default|GetInteractionWidget) false false)
        (else
          (Development|SetHiddeninGame (Variables|Default|GetInteractionWidget) true false))))))

(fn ChangeNameinWidget
  (params (Character :type Third%20Person%20Character%20Object%20Reference) (Widget%20World :type Widget%20Component%20Object%20Reference) (Widget%20Screen :type W%20Interaction%20Screen%20Object%20Reference) (Name :type Text))
  (switch Utilities|FlowControl|Switch|SwitchonEPlayer (Variables|/Game/HorrorContent/MainBlueprints/ThirdPersonCharacter.ThirdPersonCharacter_C|GetPlayerMode Character)
    (:NewEnumerator0
      (Rendering|Components|TextRender|SetText (Variables|/Game/HorrorContent/Widgets/W_InteractionScreen.W_InteractionScreen_C|GetName Widget%20Screen) Name))
    (:NewEnumerator1
      (bind _asw_interaction_world (Utilities|Casting|CastToW_InteractionWorld (UserInterface|GetUserWidgetObject Widget%20World)))
      (Rendering|Components|TextRender|SetText (Variables|/Game/HorrorContent/Widgets/W_InteractionWorld.W_InteractionWorld_C|GetName _asw_interaction_world) Name))))