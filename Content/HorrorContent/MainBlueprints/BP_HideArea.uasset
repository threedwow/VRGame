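; BP_HideArea is a hiding volume that affects whether the AI can see the player.
; Its Box overlap events cast the other actor to ThirdPersonCharacter and write its CanAISeeMe flag.
; Both begin and end overlap set the flag to false, so leaving never restores visibility, although the end-overlap comment says it should.
; The construction script scales the Box from X, Y and Z variables.
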(event OnComponentBeginOverlap(Box)
  (params (OverlappedComponent :type Primitive%20Component%20Object%20Reference) (OtherActor :type Actor%20Object%20Reference) (OtherComp :type Primitive%20Component%20Object%20Reference) (OtherBodyIndex :type Integer) (bFromSweep :type Boolean) (SweepResult :type Hit%20Result%20Structure%20%28by%20ref%29))
  ;[1 1 1] Hide Player
  (bind _asthird_person_character (Utilities|Casting|CastToThirdPersonCharacter OtherActor))
  (Variables|/Game/HorrorContent/MainBlueprints/ThirdPersonCharacter.ThirdPersonCharacter_C|SetCanAISeeMe? _asthird_person_character false))

(event OnComponentEndOverlap(Box)
  (params (OverlappedComponent :type Primitive%20Component%20Object%20Reference) (OtherActor :type Actor%20Object%20Reference) (OtherComp :type Primitive%20Component%20Object%20Reference) (OtherBodyIndex :type Integer))
  ;[1 1 1] Make Player visiable to AI
  (bind _asthird_person_character (Utilities|Casting|CastToThirdPersonCharacter OtherActor))
  (Variables|/Game/HorrorContent/MainBlueprints/ThirdPersonCharacter.ThirdPersonCharacter_C|SetCanAISeeMe? _asthird_person_character false))

(fn ConstructionScript
  (Transformation|SetRelativeScale3D (Variables|Default|GetBox) (Math|Vector|MakeVector (Variables|Scale|GetX) (Variables|Scale|GetY) (Variables|Scale|GetZ))))