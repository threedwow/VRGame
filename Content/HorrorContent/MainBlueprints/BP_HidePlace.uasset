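; BP_HidePlace is a horror-game hiding spot with a timeline-driven door and an interaction prompt for first- or third-person mode.
; Interacting opens the door, entering or leaving the hide area closes it after a delay, and door movement can emit AI-audible noise.
; Entering hides the player from AI, unless a controller is in the follow state: then the first AI character is sent to kill them and the area briefly deactivates.
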(event OnComponentBeginOverlap(AIDontSeePlayerArea)
  (params (OverlappedComponent :type Primitive%20Component%20Object%20Reference) (OtherActor :type Actor%20Object%20Reference) (OtherComp :type Primitive%20Component%20Object%20Reference) (OtherBodyIndex :type Integer) (bFromSweep :type Boolean) (SweepResult :type Hit%20Result%20Structure%20%28by%20ref%29))
  (bind _aidontseeplayerarea (Variables|Default|GetAIDontSeePlayerArea))
  ;[1 1 1] Door movement timeline
  ;[1 1 1] AI can not see player while player in these area
  (bind _asthird_person_character (Utilities|Casting|CastToThirdPersonCharacter OtherActor))
  (bind _aifollow_ (CallFunction|CheckAIFollowPlayer))
  (if _aifollow_
    ;[1 1 1] If you saw player entering some hide place go and try to kill him
    (bind _outactors (Actor|GetAllActorsOfClass "/Game/HorrorContent/AI/AI_Character.AI_Character_C"))
    (Default|GoKillPlayer (Utilities|Array|Get(acopy) _outactors) self)
    (Components|Activation|Deactivate _aidontseeplayerarea)
    (Utilities|FlowControl|Delay 1e+01)
    (Components|Activation|Activate _aidontseeplayerarea false)
    (else
      (Variables|/Game/HorrorContent/MainBlueprints/ThirdPersonCharacter.ThirdPersonCharacter_C|SetCanAISeeMe? _asthird_person_character false)
      (Variables|Default|SetUsedByPlayer? true)
      ;[1 1 1] CloseDoor
      (Utilities|FlowControl|Delay 1.0)
      (CallFunction|CloseDoor))))

(event OnComponentEndOverlap(AIDontSeePlayerArea)
  (params (OverlappedComponent :type Primitive%20Component%20Object%20Reference) (OtherActor :type Actor%20Object%20Reference) (OtherComp :type Primitive%20Component%20Object%20Reference) (OtherBodyIndex :type Integer))
  ;[1 1 1] AI can not see player while player in these area
  (bind _asthird_person_character (Utilities|Casting|CastToThirdPersonCharacter OtherActor))
  (Variables|/Game/HorrorContent/MainBlueprints/ThirdPersonCharacter.ThirdPersonCharacter_C|SetCanAISeeMe? _asthird_person_character true)
  (Variables|Default|SetUsedByPlayer? false)
  ;[1 1 1] CloseDoor
  (Utilities|FlowControl|Delay 1.0)
  (CallFunction|CloseDoor))

(event Custom|OpenDoorTimeline
  ;[1 1 1] Door movement timeline
  (Audio|PlaySound2D (Variables|Default|GetOpenDoorSound))
  (CallFunction|MakeDoorNoise (Variables|Noise|GetCanMakeNoise) (Transformation|GetActorLocation))
  (bind _value (Timeline|DoorOpenClose Play)
    (:Update
      (Transformation|SetRelativeRotation (Variables|Default|GetDoor) (Math|Rotator|MakeRotator 0.0 0.0 _value) false false)
      (Variables|Default|SetCanUseDoor? false))
    (:Finished
      (Variables|Default|SetCanUseDoor? true))))

(event Custom|CloseDoorTimeline
  ;[1 1 1] Door movement timeline
  (Audio|PlaySound2D (Variables|Default|GetCloseDoorSound))
  (CallFunction|MakeDoorNoise (Variables|Noise|GetCanMakeNoise) (Transformation|GetActorLocation))
  (bind _value (Timeline|DoorOpenClose Reverse)
    (:Update
      (Transformation|SetRelativeRotation (Variables|Default|GetDoor) (Math|Rotator|MakeRotator 0.0 0.0 _value) false false)
      (Variables|Default|SetCanUseDoor? false))
    (:Finished
      (Variables|Default|SetCanUseDoor? true))))

(event Custom|MakeDoorNoise
  (params (NeedToMakeNoise? :type Boolean) (NoiseLocation :type Vector))
  ;[1 1 1] DoorMakeNoise
  (if NeedToMakeNoise?
    (Class|Actor|MakeNoise (Variables|Noise|GetNoise) (Game|Player|GetPlayerPawn 0) NoiseLocation 0.0 "None")))

(event Custom|CloseDoor
  ;[1 1 1] Open or close door when player interact
  ;;[1 1 1] Change widgets state and close door
  (CallFunction|CloseDoorTimeline)
  (CallFunction|ChangeNameinWidget (stale EventInteractwith Character) (Variables|Default|GetInteractionWidget) (Variables|/Game/HorrorContent/MainBlueprints/ThirdPersonCharacter.ThirdPersonCharacter_C|GetInteractionWidgetScreen (stale EventInteractwith Character)) (Utilities|Array|Get(acopy) (Variables|Default|GetUseText) 1)))

(event EventPlayerEnterRadius
  (params (Character :type Third%20Person%20Character%20Object%20Reference))
  ;[1 1 1] Setting up widget depending on players state
  (if (Variables|Default|GetCanBeUsedByPlayer?)
    (CallFunction|NewWidgetState Character true)))

(event EventPlayerLeaveRadius
  (params (Chareacter :type Third%20Person%20Character%20Object%20Reference))
  ;[1 1 1] Setting up widget depending on players state
  (if (Variables|Default|GetCanBeUsedByPlayer?)
    (CallFunction|NewWidgetState Chareacter false)))

(event EventInteractwith
  (params (Character :type Third%20Person%20Character%20Object%20Reference))
  ;[1 1 1] Open or close door when player interact
  (if (Variables|Default|GetCanBeUsedByPlayer?)
    ;;[1 1 1] Player can not use door while timeline is played
    (if (Variables|Default|GetCanUseDoor?)
      ;;[1 1 1] Change widgets state and close door
      (CallFunction|OpenDoorTimeline)
      (CallFunction|ChangeNameinWidget Character (Variables|Default|GetInteractionWidget) (Variables|/Game/HorrorContent/MainBlueprints/ThirdPersonCharacter.ThirdPersonCharacter_C|GetInteractionWidgetScreen Character) (Utilities|Array|Get(acopy) (Variables|Default|GetUseText))))))

(fn ConstructionScript)

(fn NewWidgetState
  (params (Player :type Third%20Person%20Character%20Object%20Reference) (New%20hidden :type Boolean))
  ;[1 1 1] Setting up widget
  (switch Utilities|FlowControl|Switch|SwitchonEPlayer (Variables|/Game/HorrorContent/MainBlueprints/ThirdPersonCharacter.ThirdPersonCharacter_C|GetPlayerMode Player)
    (:NewEnumerator0
      ;;[1 1 1] Visibility for third person widget
      (if New%20hidden
        (Widget|SetVisibility (Variables|/Game/HorrorContent/MainBlueprints/ThirdPersonCharacter.ThirdPersonCharacter_C|GetInteractionWidgetScreen Player) "Visible")
        (else
          (Widget|SetVisibility (Variables|/Game/HorrorContent/MainBlueprints/ThirdPersonCharacter.ThirdPersonCharacter_C|GetInteractionWidgetScreen Player) "Hidden"))))
    (:NewEnumerator1
      ;;[1 1 1] Visibility for first person widget
      (if New%20hidden
        (Development|SetHiddeninGame (Variables|Default|GetInteractionWidget) false false)
        (else
          (Development|SetHiddeninGame (Variables|Default|GetInteractionWidget) true false))))))

(fn ChangeNameinWidget
  (params (Character :type Third%20Person%20Character%20Object%20Reference) (Widget%20World :type Widget%20Component%20Object%20Reference) (Widget%20Screen :type W%20Interaction%20Screen%20Object%20Reference) (Name :type Text))
  (switch Utilities|FlowControl|Switch|SwitchonEPlayer (Variables|/Game/HorrorContent/MainBlueprints/ThirdPersonCharacter.ThirdPersonCharacter_C|GetPlayerMode Character)
    (:NewEnumerator0
      (Rendering|Components|TextRender|SetText (Variables|/Game/HorrorContent/Widgets/W_InteractionScreen.W_InteractionScreen_C|GetName Widget%20Screen) Name))
    (:NewEnumerator1
      (bind _asw_interaction_world (Utilities|Casting|CastToW_InteractionWorld (UserInterface|GetUserWidgetObject Widget%20World)))
      (Rendering|Components|TextRender|SetText (Variables|/Game/HorrorContent/Widgets/W_InteractionWorld.W_InteractionWorld_C|GetName _asw_interaction_world) Name))))

(fn CheckAIFollowPlayer
  (bind _outactors (Actor|GetAllActorsOfClass "/Game/HorrorContent/AI/AI_Controller.AI_Controller_C"))
  (for _array_element _outactors
    (if (Utilities|Enum|Equal(Enum) (Variables|/Game/HorrorContent/AI/AI_Controller.AI_Controller_C|GetAI_State _array_element) "NewEnumerator3")
      (return true _array_element)))
  (return false 0))